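; BP_Player_CharTest is a player character, apparently for testing, with directional movement, a tuned jump and a horizontal dodge.
; It raises gravity at the jump apex for a faster fall, then restores it on Tick once no longer falling.
; Dodge disables the movement mode and uses a timeline to lerp the actor left or right by facing, without sweep, then restores Walking.
; Tick also runs the dodge cooldown.
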(event `self.ReceiveBeginPlay`
  (add `self.OnReachedJumpApex` (delegate `OnReachedJumpApex_Event`)))

(event `OnReachedJumpApex_Event`
  (set `CharacterMovementComponent.GravityScale` 4.5 (`self.CharacterMovement`)))

(event `self.ReceiveTick`
  (params (DeltaSeconds :type "Float (single-precision)"))
  (bind _charactermovement (`self.CharacterMovement`))
  (`|ExecutionSequence`
    (:`then_0`
      ; Handle Apex and Gravity Change
      (if (`NavMovementComponent.IsFalling` _charactermovement)
        (set `CharacterMovementComponent.bNotifyApex` true _charactermovement)
        (elif (> (`CharacterMovementComponent.GravityScale` _charactermovement) 1.0)
          (set `CharacterMovementComponent.GravityScale` 1.0 _charactermovement))))
    (:`then_1`
      (if (not (`self.IsAbleToDodge`))
        (bind _output_get (set `self.TimeSinceLastDodge` (+ (`self.TimeSinceLastDodge`) DeltaSeconds)))
        (if (>= _output_get (`self.DodgeDelay`))
          (set `self.IsAbleToDodge` true)
          (set `self.TimeSinceLastDodge` 0.0))))))

(event `PlayTimeline`
  (bind (_direction _t) (`Timeline|DashTimeline` :!via `PlayFromStart`)
    (:`Update`
      (`self.K2_SetActorLocation` (`KismetMathLibrary.VLerp` (`self.DashStartLocation`) (`self.DashTargetLocation`) _t)))
    (:`Finished`
      (`CharacterMovementComponent.SetMovementMode` (`self.CharacterMovement`) "MOVE_Walking" 0))))

(fn `Dodge`
  (if (`self.IsAbleToDodge`)
    (set `self.DashStartLocation` (`self.K2_GetActorLocation`))
    (if (`self.IsFacingRight`)
      (set `self.DashTargetLocation` (+ (`self.DashStartLocation`) (* (1.0 0.0 0.0) (`self.DodgeForce`))))
      (else
        (set `self.DashTargetLocation` (+ (`self.DashStartLocation`) (* (-1.0 0.0 0.0) (`self.DodgeForce`))))))
    (set `self.IsAbleToDodge` false)
    (`CharacterMovementComponent.SetMovementMode` (`self.CharacterMovement`) "MOVE_None" 0)
    (`self.PlayTimeline`)))

(fn `Move`
  (params (Direction :type "Vector Structure"))
  (`self.AddMovementInput` (`KismetMathLibrary.Normal` Direction)))

(fn `UserConstructionScript`)