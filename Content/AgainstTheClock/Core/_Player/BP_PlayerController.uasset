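; Player controller that turns Enhanced Input actions into commands for the BP_Player_CharTest pawn.
; BeginPlay adds the IMC_Player mapping context and caches the cast controlled pawn, logging a message if the cast fails.
; Move input sets the pawn's facing flag from the axis sign and moves it along world X, scaled by MoveSpeed.
; Jump and Dodge presses forward directly to the pawn.
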(event `self.ReceiveBeginPlay`
  (`EnhancedInputSubsystemInterface.AddMappingContext` (pcsubsystem `EnhancedInputLocalPlayerSubsystem` self) "/Game/AgainstTheClock/Input/IMC_Player.IMC_Player" 0 (struct))
  (bind _asbp_player_char_test (cast `/Game/AgainstTheClock/Core/_Player/BP_Player_CharTest` (`self.K2_GetPawn`))
    (:`then`
      (set `self.M_ControlledPawn` _asbp_player_char_test))
    (:`CastFailed`
      (`KismetSystemLibrary.LogString` "Failed to Cast/Find controlled Pawn"))))

(event `EnhancedInput|/Game/AgainstTheClock/Input/IA_Move`
  (params (ActionValue :type "Float (double-precision)") (ElapsedSeconds :type "Float (double-precision)") (TriggeredSeconds :type "Float (double-precision)") (InputAction :type "InputAction Object Reference" :default "/Game/AgainstTheClock/Input/IA_Move.IA_Move"))
  (bind _m_controlledpawn (`self.M_ControlledPawn`))
  (:`Triggered`
    (if (> ActionValue 0.0)
      (set `/Game/AgainstTheClock/Core/_Player/BP_Player_CharTest.IsFacingRight` true _m_controlledpawn)
      (else
        (set `/Game/AgainstTheClock/Core/_Player/BP_Player_CharTest.IsFacingRight` false _m_controlledpawn)))
    (`/Game/AgainstTheClock/Core/_Player/BP_Player_CharTest.Move` (`self.M_ControlledPawn`) (* (* (1.0 0.0 0.0) ActionValue) (`self.MoveSpeed`)))))

(event `EnhancedInput|/Game/AgainstTheClock/Input/IA_Jump`
  (params (ActionValue :type Boolean) (ElapsedSeconds :type "Float (double-precision)") (TriggeredSeconds :type "Float (double-precision)") (InputAction :type "InputAction Object Reference" :default "/Game/AgainstTheClock/Input/IA_Jump.IA_Jump"))
  (:`Started`
    (`Character.Jump` (`self.M_ControlledPawn`))))

(event `EnhancedInput|/Game/AgainstTheClock/Input/IA_Dodge`
  (params (ActionValue :type Boolean) (ElapsedSeconds :type "Float (double-precision)") (TriggeredSeconds :type "Float (double-precision)") (InputAction :type "InputAction Object Reference" :default "/Game/AgainstTheClock/Input/IA_Dodge.IA_Dodge"))
  (:`Started`
    (`/Game/AgainstTheClock/Core/_Player/BP_Player_CharTest.Dodge` (`self.M_ControlledPawn`))))

(fn `UserConstructionScript`)