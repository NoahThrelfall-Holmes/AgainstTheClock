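; BP_Projectile_Base is a projectile actor in the boss clock folder that damages the player on overlap.
; While moving and the player's temporary game-running flag is set, it advances each Tick along its negative forward vector with a swept SetActorLocation, adding Speed per frame without delta-time scaling.
; Overlapping an actor whose class is exactly BP_Player_CharTest applies BaseDamage through that actor's BP_HealthComponent.
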(event `self.ReceiveBeginPlay`
  (bind _returnvalue (`GameplayStatics.GetActorOfClass` "/Game/AgainstTheClock/Core/_Player/BP_Player_CharTest.BP_Player_CharTest_C"))
  (set `self.TEMP_Player` _returnvalue))

(event `self.ReceiveTick`
  (params (DeltaSeconds :type "Float (single-precision)"))
  (bind _returnvalue_location (`KismetMathLibrary.BreakTransform` (`self.GetTransform`)))
  (if (`self.IsMoving`)
    (if (`/Game/AgainstTheClock/Core/_Player/BP_Player_CharTest.TEMP_GameRuning` (`self.TEMP_Player`))
      (`self.K2_SetActorLocation` (+ _returnvalue_location (* (* (`self.GetActorForwardVector`) -1.0) (`self.Speed`))) true))))

(event `self.ReceiveActorBeginOverlap`
  (params (OtherActor :type "Actor Object Reference"))
  (if (== (`GameplayStatics.GetObjectClass` OtherActor) "/Game/AgainstTheClock/Core/_Player/BP_Player_CharTest.BP_Player_CharTest_C")
    (`/Game/AgainstTheClock/Core/Components/BP_HealthComponent.TakeDamage` (`self.GetComponentByClass` OtherActor "/Game/AgainstTheClock/Core/Components/BP_HealthComponent.BP_HealthComponent_C") (`self.BaseDamage`))))

(fn `UserConstructionScript`)